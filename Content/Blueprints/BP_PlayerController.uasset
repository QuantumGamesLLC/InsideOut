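; Player controller that turns touch swipes and taps into movement commands for the BP_Sphere pawn.
; Once a drag's squared length exceeds SwipeThreshold, a DoOnce gate sets the pawn's Direction from the dominant axis and sign, without waiting for release.
; Releasing the touch re-arms the gate, and a release almost at the start point teleports the pawn to the world origin.
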(event `InputTouch`
  (params (Location :type "Vector Structure") (FingerIndex :type "ETouchIndex Enum"))
  (bind _asbp_sphere (`self.GetControlledPawn`))
  (bind _x (.x (- (`self.StartTouchLocation`) (`self.EndSwipeLocation`))))
  (bind _y (.y (- (`self.StartTouchLocation`) (`self.EndSwipeLocation`))))
  (:`Pressed`
    (set `self.StartTouchLocation` Location))
  (:`Released`
    (`|ExecutionSequence`
      (:`then_0`
        (goto _label :!via `Reset`))
      (:`then_1`
        (if (== (`self.StartTouchLocation`) Location :`ErrorTolerance` 2.0)
          (`self.K2_SetActorLocation` (`self.GetControlledPawn`) (0.0 0.0 0.0) false true)))))
  (:`Moved`
    (if (> (`KismetMathLibrary.VSizeSquared` (- (`self.StartTouchLocation`) Location)) (`self.SwipeThreshold`))
      (`/Engine/EditorBlueprintResources/StandardMacros.DoOnce` false :!label _label
        (:`Completed`
          (set `self.EndSwipeLocation` Location)
          (if (> (`KismetMathLibrary.Abs` _x) (`KismetMathLibrary.Abs` _y))
            (if (> _x 0.0)
              (set `/Game/Blueprints/BP_Sphere.Direction` "NewEnumerator1" _asbp_sphere)
              (else
                (set `/Game/Blueprints/BP_Sphere.Direction` "NewEnumerator0" _asbp_sphere)))
            (elif (> _y 0.0)
              (set `/Game/Blueprints/BP_Sphere.Direction` "NewEnumerator2" _asbp_sphere)
              (else
                (set `/Game/Blueprints/BP_Sphere.Direction` "NewEnumerator3" _asbp_sphere)))))))))

(fn `GetControlledPawn`
  (returns (`AsBP Sphere` :type "/Game/Blueprints/BP_Sphere Object Reference"))
  (bind _asbp_sphere (cast `/Game/Blueprints/BP_Sphere` (`self.K2_GetPawn`))
    (:`then`
      (return _asbp_sphere))
    (:`CastFailed`
      (return null))))

(fn `UserConstructionScript`)